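; Manager actor for a cube-shooting game that keeps one moving cube spawning after another until the target count is shot.
; Each BP_MovingCube gets a random navmesh-reachable XY, random height, axis-aligned velocity, size and travel distance, using ranges partly from BP_GameInstanc.
; OnCubeDestroyed updates the game mode's count, then spawns again or finishes the round.
; Finishing writes cached cube statistics to a hard-coded desktop folder and opens the Start level.
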(event `self.ReceiveBeginPlay`
  (`self.SpawnMovingCube`))

(event `OnCubeDestroyed`
  (bind _returnvalue (subsystem `StatisticsSubsystem`))
  (`/Engine/EditorBlueprintResources/StandardMacros.IncrementInt` (`self.NumCubesShot`)
    (:`  `
      (bind _asbp_first_person_game_mode (cast `/Game/BallGame/core/BP_FirstPersonGameMode` (`GameplayStatics.GetGameMode`)))
      (`/Game/BallGame/core/BP_FirstPersonGameMode.OnCubeShot` _asbp_first_person_game_mode (`self.NumCubesShot`))
      (bind _asbp_game_instanc (cast `/Game/BallGame/core/BP_GameInstanc` (`GameplayStatics.GetGameInstance`)))
      (if (>= (`self.NumCubesShot`) (`/Game/BallGame/core/BP_GameInstanc.NumCubesToShoot` _asbp_game_instanc))
        (`StatisticsSubsystem.SetFilePath` _returnvalue "C:\\\\Users\\\\Christina\\\\Desktop\\\\BallGameStatistics\\\\")
        (`StatisticsSubsystem.WriteCachedCubeInfo` _returnvalue)
        (`GameplayStatics.OpenLevelBySoftObjectPtr` "/Game/Maps/Start.Start")
        (else
          (`self.SpawnMovingCube`))))))

(fn `GetRandomSize`
  (returns (Size :type "Vector Structure"))
  (bind _asbp_game_instanc (cast `/Game/BallGame/core/BP_GameInstanc` (`GameplayStatics.GetGameInstance`)))
  (bind _returnvalue (`KismetMathLibrary.RandomFloatInRange` (`/Game/BallGame/core/BP_GameInstanc.CubeSizeMin` _asbp_game_instanc) (`/Game/BallGame/core/BP_GameInstanc.CubeSizeMax` _asbp_game_instanc)))
  (return (`KismetMathLibrary.MakeVector` _returnvalue _returnvalue _returnvalue)))

(fn `GetRandomSpawnTransform`
  (returns (SpawnTransform :type "Transform Structure"))
  (bind _randomlocation (`NavigationSystemV1.K2_GetRandomReachablePointInRadius` (`self.K2_GetActorLocation`) 3000.0 null null))
  (`KismetSystemLibrary.PrintString` (`KismetStringLibrary.Concat_StrStr` (`KismetStringLibrary.Conv_DoubleToString` (.x _randomlocation)) (`KismetStringLibrary.Conv_DoubleToString` (.y _randomlocation))))
  (return (`KismetMathLibrary.MakeTransform` (`KismetMathLibrary.MakeVector` (.x _randomlocation) (.y _randomlocation) (`KismetMathLibrary.RandomFloatInRange` 200.0 500.0)))))

(fn `GetRandomVelocity`
  (returns (Velocity :type "Vector Structure"))
  (bind _asbp_game_instanc (cast `/Game/BallGame/core/BP_GameInstanc` (`GameplayStatics.GetGameInstance`)))
  (return (* (select `int` (`KismetMathLibrary.RandomIntegerInRange` 0 2) :`0` (`KismetMathLibrary.MakeVector` 1.0) :`1` (`KismetMathLibrary.MakeVector` 0.0 1.0) :`2` (`KismetMathLibrary.MakeVector` 0.0 0.0 1.0)) (`KismetMathLibrary.RandomFloatInRange` (`/Game/BallGame/core/BP_GameInstanc.CubeSpeedMin` _asbp_game_instanc) (`/Game/BallGame/core/BP_GameInstanc.CubeSpeedMax` _asbp_game_instanc)))))

(fn `SpawnMovingCube`
  (`|SpawnActorFromClass` "/Game/BallGame/BP_MovingCube.BP_MovingCube_C" (`self.GetRandomSpawnTransform`) "Undefined" "OverrideRootScale" null (`self.GetRandomVelocity`) (`self.GetRandomSize`) (`KismetMathLibrary.RandomFloatInRange` 70.0 500.0) null))

(fn `UserConstructionScript`)