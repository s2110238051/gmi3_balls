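; BP_TeleportComponent is a component that lets its owning actor teleport to a point it aims at.
; On BeginPlay it spawns a BP_TeleportTarget marker, whose sphere shows between StartTeleport and EndTeleport.
; While aiming, Tick line-traces along the component's forward vector, projects the hit onto the navmesh and moves the marker there.
; EndTeleport hides the marker and, if the trace hit, moves the owner to that XY, keeping its current Z.
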(event `self.ReceiveBeginPlay`
  (set `self.ActorToBeTeleported` (`self.GetOwner`))
  (bind _returnvalue (`|SpawnActorFromClass` "/Game/BallGame/BP_TeleportTarget.BP_TeleportTarget_C" (`KismetMathLibrary.MakeTransform` (0.0 0.0 0.0)) "Undefined" "OverrideRootScale" null null))
  (set `self.TargetAcotr` _returnvalue))

(event `self.ReceiveTick`
  (params (DeltaSeconds :type "Float (single-precision)"))
  (if (`self.bIsTeleporting`)
    (`self.DetectHitPoint`)))

(fn `DetectHitPoint`
  (bind _returnvalue (`self.K2_GetComponentLocation`))
  (bind (_outhit _returnvalue_2) (`KismetSystemLibrary.LineTraceSingle` _returnvalue (+ _returnvalue (* (`self.GetForwardVector`) (`self.distance`))) "TraceTypeQuery1"))
  (bind _projectedlocation (`NavigationSystemV1.K2_ProjectPointToNavigation` (`.Location` (`GameplayStatics.BreakHitResult` _outhit))))
  (set `self.HitLocation` _projectedlocation)
  (bind _output_get (set `self.bHitDetected` _returnvalue_2))
  (if _output_get
    (`Actor.K2_SetActorLocation` (`self.TargetAcotr`) _projectedlocation false false)))

(fn `EndTeleport`
  (bind (_hitlocation_x _hitlocation_y) (`KismetMathLibrary.BreakVector` (`self.HitLocation`)))
  (bind (_returnvalue_x _returnvalue_y _returnvalue_z) (`KismetMathLibrary.BreakVector` (`Actor.K2_GetActorLocation` (`self.ActorToBeTeleported`))))
  (set `self.bIsTeleporting` false)
  (`self.SetVisibility` (`/Game/BallGame/BP_TeleportTarget.Sphere` (`self.TargetAcotr`)) false false)
  (if (`self.bHitDetected`)
    (`Actor.K2_SetActorLocation` (`self.ActorToBeTeleported`) (`KismetMathLibrary.MakeVector` _hitlocation_x _hitlocation_y _returnvalue_z) false false)))

(fn `StartTeleport`
  (bind _output_get (set `self.bIsTeleporting` true))
  (`self.SetVisibility` (`/Game/BallGame/BP_TeleportTarget.Sphere` (`self.TargetAcotr`)) _output_get false))